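; Door actor that slides open when the player, inside its trigger box, presses E at a "Press E to Show ID" prompt.
; Box overlap enables and disables input for the ThirdPersonCharacter's player, with the prompt shown via PrintString.
; E plays door audio, then after a one-second delay runs a timeline lerping Cube between Start and End; Q reverses it.
; A Moving flag set by the timeline blocks input mid-motion.
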(event OnComponentBeginOverlap(Box)
  (params (OverlappedComponent :type Primitive%20Component%20Object%20Reference) (OtherActor :type Actor%20Object%20Reference) (OtherComp :type Primitive%20Component%20Object%20Reference) (OtherBodyIndex :type Integer) (bFromSweep :type Boolean) (SweepResult :type Hit%20Result%20Structure%20%28by%20ref%29))
  ;[1 1 1] Input for the player
  (Utilities|Casting|CastToThirdPersonCharacter OtherActor)
  (Input|EnableInput (Game|GetPlayerController 0))
  (Development|PrintString "Press E to Show ID"))

(event OnComponentEndOverlap(Box)
  (params (OverlappedComponent :type Primitive%20Component%20Object%20Reference) (OtherActor :type Actor%20Object%20Reference) (OtherComp :type Primitive%20Component%20Object%20Reference) (OtherBodyIndex :type Integer))
  ;[1 1 1] Input for the player
  (Utilities|Casting|CastToThirdPersonCharacter OtherActor)
  (Input|DisableInput (Game|GetPlayerController 0)))

(event Input|KeyboardEvents|E
  (params (Key :type Key%20Structure))
  ;[1 1 1] Input of Q and E to make the platform move up or down
  ;;[1 0.1371 0.04746] Sets the movement keys
  (:Pressed
    (if (not (Variables|Default|GetMoving))
      (Utilities|FlowControl|Sequence
        (:then_0
          ;[0.2708 0.3543 1] Audio for the door opening
          (bind _returnvalue (AddComponent|AddAudioComponent false))
          (Audio|Components|Audio|Play _returnvalue 0.0))
        (:then_1
          (Utilities|FlowControl|Delay 1.0)
          ;;[1 0.8863 0.3198] Plays the start and end locations for the door
          (bind _alpha (Timeline|Timeline_0 Play)
            (:Update
              (Variables|Default|SetMoving true)
              (Transformation|SetRelativeLocation (Variables|Default|GetCube) (Math|Vector|Lerp(Vector) (Variables|Default|GetStart) (Variables|Default|GetEnd) _alpha) false false))
            (:Finished
              (Variables|Default|SetMoving false))))))))

(event Input|KeyboardEvents|Q
  (params (Key :type Key%20Structure))
  ;[1 1 1] Input of Q and E to make the platform move up or down
  ;;[1 0.1371 0.04746] Sets the movement keys
  (:Pressed
    (if (not (Variables|Default|GetMoving))
      ;;[1 0.8863 0.3198] Plays the start and end locations for the door
      (bind _alpha (Timeline|Timeline_0 Reverse)
        (:Update
          (Variables|Default|SetMoving true)
          (Transformation|SetRelativeLocation (Variables|Default|GetCube) (Math|Vector|Lerp(Vector) (Variables|Default|GetStart) (Variables|Default|GetEnd) _alpha) false false))
        (:Finished
          (Variables|Default|SetMoving false))))))

(fn ConstructionScript)