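; Pressure plate that toggles its own on/off state when the third-person character steps on it, in the style of a Lights Out switch puzzle.
; Each overlap of its Box also flips the state of every plate in its Pads array, then adds and plays an audio component.
; Tick reapplies the Blue or Bottle material to the Cube every frame to show the current state.
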(event OnComponentBeginOverlap(Box)
  (params (OverlappedComponent :type Primitive%20Component%20Object%20Reference) (OtherActor :type Actor%20Object%20Reference) (OtherComp :type Primitive%20Component%20Object%20Reference) (OtherBodyIndex :type Integer) (bFromSweep :type Boolean) (SweepResult :type Hit%20Result%20Structure%20%28by%20ref%29))
  ;[1 1 1] Interacts with the third person character
  (if true
    ;[1 1 1] sets up the array to see if the switches get turned on or off when the player steps on one
    (if (== (Utilities|GetClass OtherActor) "/Game/ThirdPersonBP/Blueprints/ThirdPersonCharacter.ThirdPersonCharacter_C")
      ;[0.3873 0.4415 1] Plays the audio for when the player steps on one of the pick ups
      (Utilities|FlowControl|Sequence
        (:then_0
          (if (Variables|Default|GetActiveState)
            ;;[1 0.2341 0.1043] Sets up the array for the pads to know who to turn on
            (Variables|Default|SetActiveState false)
            (else
              (Variables|Default|SetActiveState true)))
          (for _array_element (Variables|Default|GetPads)
            (if (Variables|Plates_BP_C|GetActiveState _array_element)
              (Variables|Plates_BP_C|SetActiveState _array_element false)
              (else
                (Variables|Plates_BP_C|SetActiveState _array_element true)))))
        (:then_1
          (bind _returnvalue (AddComponent|AddAudioComponent false))
          (Audio|Components|Audio|Play _returnvalue 0.0))))))

(event EventTick
  (params (DeltaSeconds :type Float%20%28single-precision%29))
  (bind _cube (Variables|Default|GetCube))
  ;[1 1 1] Sets the colour of the pads when they get stepped on
  (if (Variables|Default|GetActiveState)
    (Rendering|Material|SetMaterial _cube 0 "/Game/Textures/Blue.Blue")
    (else
      (Rendering|Material|SetMaterial _cube 0 "/Game/Textures/Bottle.Bottle"))))

(fn ConstructionScript)