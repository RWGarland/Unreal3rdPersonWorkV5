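; Third-person game mode that runs a countdown and ends the game when time runs out.
; Tick feeds a one-second Delay, which throttles the Seconds decrement to roughly once per second.
; At zero it prints a game-over message, spawns a GameOver actor at the player character's transform, then pauses the game after a short delay.
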(event EventTick
  (params (DeltaSeconds :type Float%20%28single-precision%29))
  (Utilities|FlowControl|Delay 1.0)
  (if (> (Variables|Default|GetSeconds) 0)
    (Variables|Default|SetSeconds (- (Variables|Default|GetSeconds) 1))
    (else
      (Development|PrintString "Game Over")
      (Game|SpawnActorfromClass "/Game/Blueprints/GameOver.GameOver_C" (Transformation|GetActorTransform (Game|GetPlayerCharacter 0)) "Undefined" 0 0)
      (Utilities|FlowControl|Delay 1.0)
      (Game|SetGamePaused true))))

(fn ConstructionScript)