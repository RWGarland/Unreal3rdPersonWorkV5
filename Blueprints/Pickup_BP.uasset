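; A score pickup actor that the player's ThirdPersonCharacter collects by overlapping it.
; On overlap it destroys itself, adds points to the Score in MyGameInstance_BP and calls NextPickup on the first Spawner_BP found in the level.
; It also plays a sound through an audio component added after the destroy call.
; Uncollected pickups destroy themselves after a long Delay driven from Tick.
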(event EventTick
  (params (DeltaSeconds :type Float%20%28single-precision%29))
  ;[1 1 1] Timed delay before it gets destroid
  (Utilities|FlowControl|Delay 3.6e+02)
  (Actor|DestroyActor))

(event Collision|EventActorBeginOverlap
  (params (OtherActor :type Actor%20Object%20Reference))
  ;[1 1 1] Getting points when the player goes into the pickup
  (Utilities|Casting|CastToThirdPersonCharacter OtherActor)
  (Actor|DestroyActor)
  (Utilities|FlowControl|Sequence
    (:then_0
      ;[0.2874 1 0.1875] When the player hits a pick up 10 points is added to the score
      (bind _asmy_game_instance_bp (Utilities|Casting|CastToMyGameInstance_BP (Game|GetGameInstance)))
      (Variables|/Game/Blueprints/MyGameInstance_BP.MyGameInstance_BP_C|SetScore _asmy_game_instance_bp (+ (Variables|/Game/Blueprints/MyGameInstance_BP.MyGameInstance_BP_C|GetScore _asmy_game_instance_bp) 10))
      ;;[0.2912 0.2907 1] Gets the array of pickups to then know where the nect one is going to spawn
      (bind _outactors (Actor|GetAllActorsOfClass "/Game/Blueprints/Spawner_BP.Spawner_BP_C"))
      (Default|NextPickup (Utilities|Array|Get(acopy) _outactors)))
    (:then_1
      ;;[1 0 0.6864] Play Sound for pickups
      (bind _returnvalue (AddComponent|AddAudioComponent false))
      (Audio|Components|Audio|Play _returnvalue 0.0))))

(fn ConstructionScript)