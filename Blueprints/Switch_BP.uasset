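; Switch_BP is a puzzle switch that reacts when a specific block, BlockSwitch_BP, overlaps its box.
; The correct block destroys the Cube platform component to drop another cube, turns the switch mesh green and plays a sound.
; Other overlaps are filtered by casts: BlockSwitch_BP_2 and BlockSwitch_BP_3 play a wrong-block sound, while the player character only prints a debug message.
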(event OnComponentBeginOverlap(Box)
  (params (OverlappedComponent :type Primitive%20Component%20Object%20Reference) (OtherActor :type Actor%20Object%20Reference) (OtherComp :type Primitive%20Component%20Object%20Reference) (OtherBodyIndex :type Integer) (bFromSweep :type Boolean) (SweepResult :type Hit%20Result%20Structure%20%28by%20ref%29))
  ;[0.9357 1 0.4214] the switch is set to over lap with the BlockSwitch_BP
  (Utilities|FlowControl|Sequence
    (:then_0
      (bind _asblock_switch_bp (Utilities|Casting|CastToBlockSwitch_BP OtherActor)))
    (:then_1
      (if (== OtherActor _asblock_switch_bp)
        ;[1 1 1] When its the correct cube in the colision box for the switch
        (Development|PrintString "Blue Box Is now trigger")
        (Utilities|FlowControl|Sequence
          (:then_0
            ;;[1 0.1453 0.1751] Destroys platform to make the red cube fall
            (Components|DestroyComponent (Variables|Default|GetCube)))
          (:then_1
            ;;[0.1415 1 0.4903] Sets Material
            (Rendering|Material|SetMaterial (Variables|Debug|GetStaticMeshComponent) 0 "/Game/Textures/Green.Green"))
          (:then_2
            ;;[0.2622 0.2689 1] Plays the audio
            (Development|PrintString "Play sound")
            (bind _returnvalue (AddComponent|AddAudioComponent false))
            (Audio|Components|Audio|Play _returnvalue 0.0)))
        (else
          (Utilities|FlowControl|Sequence
            (:then_0
              ;[1 1 1] If anything other than the right cube goes onto the switch
              (Utilities|Casting|CastToThirdPersonCharacter OtherActor)
              ;;[0.315 1 0.9001] Wont play anything if the player walks on it
              (Development|PrintString "Wont Play anything"))
            (:then_1
              (Utilities|Casting|CastToBlockSwitch_BP_2 OtherActor)
              ;;[0.2711 0.2828 1] Plays audio for the wrong blocks
              (Development|PrintString "Play Wrong Sound" :!label _label)
              (bind _returnvalue_2 (AddComponent|AddAudioComponent false))
              (Audio|Components|Audio|Play _returnvalue_2 0.0))
            (:then_2
              (Utilities|Casting|CastToBlockSwitch_BP_3 OtherActor)
              (goto _label))))))))

(fn ConstructionScript)