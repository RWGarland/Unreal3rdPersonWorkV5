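; Elevator actor that the third-person character rides between a Start and an End position.
; Overlapping the Box trigger enables input and prints a prompt; leaving it disables input.
; E plays and Q reverses a timeline that lerps the Cube's relative location, with a Moving flag blocking both mid-travel.
; Each E press also adds and plays an audio component, even while moving.
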(event OnComponentBeginOverlap(Box)
  (params (OverlappedComponent :type Primitive%20Component%20Object%20Reference) (OtherActor :type Actor%20Object%20Reference) (OtherComp :type Primitive%20Component%20Object%20Reference) (OtherBodyIndex :type Integer) (bFromSweep :type Boolean) (SweepResult :type Hit%20Result%20Structure%20%28by%20ref%29))
  ;[1 1 1] Input for the player
  (Utilities|Casting|CastToThirdPersonCharacter OtherActor)
  (Input|EnableInput (Game|GetPlayerController 0))
  (Development|PrintString "Press E to go up"))

(event OnComponentEndOverlap(Box)
  (params (OverlappedComponent :type Primitive%20Component%20Object%20Reference) (OtherActor :type Actor%20Object%20Reference) (OtherComp :type Primitive%20Component%20Object%20Reference) (OtherBodyIndex :type Integer))
  ;[1 1 1] Input for the player
  (Utilities|Casting|CastToThirdPersonCharacter OtherActor)
  (Input|DisableInput (Game|GetPlayerController 0)))

(event Input|KeyboardEvents|E
  (params (Key :type Key%20Structure))
  ;[1 1 1] Input to make the elevator go up and down
  ;;[1 0.1354 0.1354] Input for the Player
  (:Pressed
    (Utilities|FlowControl|Sequence
      (:then_0
        (if (not (Variables|Default|GetMoving))
          ;[1 0.8941 0.2663] Plays the vectors for the lift so it can go up and down
          (bind _alpha (Timeline|Moving%20Up%20and%20down Play)
            (:Update
              (Variables|Default|SetMoving true)
              (Transformation|SetRelativeLocation (Variables|Default|GetCube) (Math|Vector|Lerp(Vector) (Variables|Default|GetStart) (Variables|Default|GetEnd) _alpha) false false))
            (:Finished
              (Variables|Default|SetMoving false)))))
      (:then_1
        ;[0.003805 1 0.8903] Plays Sound
        (bind _returnvalue (AddComponent|AddAudioComponent false))
        (Audio|Components|Audio|Play _returnvalue 0.0)))))

(event Input|KeyboardEvents|Q
  (params (Key :type Key%20Structure))
  ;[1 1 1] Input to make the elevator go up and down
  ;;[1 0.1354 0.1354] Input for the Player
  (:Pressed
    (if (not (Variables|Default|GetMoving))
      ;[1 0.8941 0.2663] Plays the vectors for the lift so it can go up and down
      (bind _alpha (Timeline|Moving%20Up%20and%20down Reverse)
        (:Update
          (Variables|Default|SetMoving true)
          (Transformation|SetRelativeLocation (Variables|Default|GetCube) (Math|Vector|Lerp(Vector) (Variables|Default|GetStart) (Variables|Default|GetEnd) _alpha) false false))
        (:Finished
          (Variables|Default|SetMoving false))))))

(fn ConstructionScript)