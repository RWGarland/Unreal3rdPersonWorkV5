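; Spawner actor that places Pickup_BP actors one at a time at the transforms of the actors in its Pickups list.
; BeginPlay spawns the first pickup at the Current index.
; The NextPickup event increments Current and spawns the next one, wrapping back to the start of the list after the last entry.
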(event Custom|NextPickup
  (bind _pickups (Variables|Default|GetPickups))
  (bind _result (Math|Integer|IncrementInt (Variables|Default|GetCurrent))
    (:%20%20
      (if (< _result (Utilities|Array|Length _pickups))
        _
        (else
          (Variables|Default|SetCurrent 0)))
      (Game|SpawnActorfromClass "/Game/Pickup_BP.Pickup_BP_C" (Transformation|GetActorTransform (Utilities|Array|Get(acopy) _pickups (Variables|Default|GetCurrent))) "Undefined" 0 0))))

(event EventBeginPlay
  (Game|SpawnActorfromClass "/Game/Pickup_BP.Pickup_BP_C" (Transformation|GetActorTransform (Utilities|Array|Get(acopy) (Variables|Default|GetPickups) (Variables|Default|GetCurrent))) "Undefined" 0 0))

(fn ConstructionScript)