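; Door Blueprint that slides a Cube between Start and End positions when the player presses keys nearby.
; A Box trigger enables input and prints an ID prompt when a ThirdPersonCharacter enters, and disables input on exit.
; E plays and Q reverses a timeline that lerps the Cube's relative location, with a Moving flag blocking new presses until it finishes.
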(event OnComponentBeginOverlap(Box)
  (params (OverlappedComponent :type Primitive%20Component%20Object%20Reference) (OtherActor :type Actor%20Object%20Reference) (OtherComp :type Primitive%20Component%20Object%20Reference) (OtherBodyIndex :type Integer) (bFromSweep :type Boolean) (SweepResult :type Hit%20Result%20Structure%20%28by%20ref%29))
  ;[1 1 1] Input for the player
  (Utilities|Casting|CastToThirdPersonCharacter OtherActor)
  (Input|EnableInput (Game|GetPlayerController 0))
  (Development|PrintString "Press E to Show ID"))

(event OnComponentEndOverlap(Box)
  (params (OverlappedComponent :type Primitive%20Component%20Object%20Reference) (OtherActor :type Actor%20Object%20Reference) (OtherComp :type Primitive%20Component%20Object%20Reference) (OtherBodyIndex :type Integer))
  ;[1 1 1] Input for the player
  (Utilities|Casting|CastToThirdPersonCharacter OtherActor)
  (Input|DisableInput (Game|GetPlayerController 0)))

(event Input|KeyboardEvents|E
  (params (Key :type Key%20Structure))
  ;[1 1 1] Input of Q and E to make the platform move up or down
  (:Pressed
    (if (not (Variables|Default|GetMoving))
      (bind _alpha (Timeline|Timeline_0 Play)
        (:Update
          (Variables|Default|SetMoving true)
          (Transformation|SetRelativeLocation (Variables|Default|GetCube) (Math|Vector|Lerp(Vector) (Variables|Default|GetStart) (Variables|Default|GetEnd) _alpha) false false))
        (:Finished
          (Variables|Default|SetMoving false))))))

(event Input|KeyboardEvents|Q
  (params (Key :type Key%20Structure))
  ;[1 1 1] Input of Q and E to make the platform move up or down
  (:Pressed
    (if (not (Variables|Default|GetMoving))
      (bind _alpha (Timeline|Timeline_0 Reverse)
        (:Update
          (Variables|Default|SetMoving true)
          (Transformation|SetRelativeLocation (Variables|Default|GetCube) (Math|Vector|Lerp(Vector) (Variables|Default|GetStart) (Variables|Default|GetEnd) _alpha) false false))
        (:Finished
          (Variables|Default|SetMoving false))))))

(fn ConstructionScript)