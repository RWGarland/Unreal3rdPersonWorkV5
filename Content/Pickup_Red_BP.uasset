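; Red pickup actor that scores a point when a ThirdPersonCharacter overlaps it.
; On overlap it destroys itself, increments Score on MyGameInstance_BP and spawns a Pickup_Blue_BP at TargetPoint2's transform.
; A Delay on Tick also destroys it after a few seconds, in which case no point is added and no blue pickup spawns.
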(event EventTick
  (params (DeltaSeconds :type Float%20%28single-precision%29))
  (Utilities|FlowControl|Delay 5.0)
  (Actor|DestroyActor))

(event Collision|EventActorBeginOverlap
  (params (OtherActor :type Actor%20Object%20Reference))
  (Utilities|Casting|CastToThirdPersonCharacter OtherActor)
  (Actor|DestroyActor)
  (bind _asmy_game_instance_bp (Utilities|Casting|CastToMyGameInstance_BP (Game|GetGameInstance)))
  (Variables|/Game/Blueprints/MyGameInstance_BP.MyGameInstance_BP_C|SetScore _asmy_game_instance_bp (+ (Variables|/Game/Blueprints/MyGameInstance_BP.MyGameInstance_BP_C|GetScore _asmy_game_instance_bp) 1))
  (Game|SpawnActorfromClass "/Game/Pickup_Blue_BP.Pickup_Blue_BP_C" (Transformation|GetActorTransform (Variables|Default|GetTargetPoint2)) "Undefined" 0 0))

(fn ConstructionScript
  (|CallParentFunction))